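; BP_Camera is a camera actor that orbits vertically around a LookAtTarget, with scroll input controlling its pitch.
; On BeginPlay it records its distance and pitch to the target, snaps to face it and adds the Enhanced Input mapping context.
; Scroll adjusts a clamped destination pitch.
; Tick interpolates toward that pitch and uses sine and cosine to place the camera at constant distance in the target's YZ plane.
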(event Input|EnhancedActionEvents|EnhancedInputActionScroll
  (params (ActionValue :type Float%20%28double-precision%29) (ElapsedSeconds :type Float%20%28double-precision%29) (TriggeredSeconds :type Float%20%28double-precision%29) (InputAction :type Input%20Action%20Object%20Reference :default "/Game/Catfishing/Assets/Input/Scroll.Scroll"))
  (:Triggered
    (Variables|Default|SetDestinationPitchAngle (Math|Float|ClampAngle (- (Variables|Default|GetDestinationPitchAngle) (* ActionValue (Variables|Default|GetScrollSensitivity) -1.0)) 2e+01 89.0))))

(event EventBeginPlay
  (bind _returnvalue (Game|GetPlayerController 0))
  (bind _returnvalue_2 (Transformation|GetActorLocation))
  (bind _returnvalue_3 (Transformation|GetActorRotation))
  (bind _lookattarget (Variables|Default|GetLookAtTarget))
  (bind _returnvalue_4 (Transformation|GetActorLocation _lookattarget))
  (bind (_roll _pitch _yaw) (Math|Rotator|BreakRotator _returnvalue_3))
  (bind _returnvalue_5 (PlayerController|LocalPlayerSubsystems|GetEnhancedInputLocalPlayerSubsystem _returnvalue))
  (bind _returnvalue_6 (Math|Rotator|FindLookatRotation _returnvalue_2 _returnvalue_4))
  (bind _pitch_2 (Math|Rotator|BreakRotator _returnvalue_6))
  (Variables|Default|SetDistanceFromTarget (Math|Vector|Distance(Vector) _returnvalue_2 _returnvalue_4))
  (Variables|Default|SetDestinationPitchAngle (* _pitch_2 -1.0))
  (Transformation|SetActorRotation (Math|Rotator|MakeRotator _roll _pitch_2 _yaw))
  (Utilities|IsValid _returnvalue_5
    (:Is%20Valid
      (Input|AddMappingContext _returnvalue_5 "/Game/Catfishing/Assets/Input/InputMapping.InputMapping" 0 "(bIgnoreAllPressedKeysUntilRelease=True,bForceImmediately=False)"))))

(event EventTick
  (params (DeltaSeconds :type Float%20%28single-precision%29))
  (bind _returnvalue (Transformation|GetActorRotation))
  (bind _destinationpitchangle (Variables|Default|GetDestinationPitchAngle))
  (bind _cameraspeed (Variables|Default|GetCameraSpeed))
  (bind _distancefromtarget (Variables|Default|GetDistanceFromTarget))
  (bind (_roll _pitch _yaw) (Math|Rotator|BreakRotator _returnvalue))
  (bind _returnvalue_2 (* _destinationpitchangle -1.0))
  (bind _returnvalue_3 (Math|Interpolation|FInterpTo _pitch _returnvalue_2 DeltaSeconds _cameraspeed))
  (Transformation|SetActorRotation (Math|Rotator|MakeRotator _roll _returnvalue_3 _yaw))
  (Transformation|SetActorLocation (+ (Transformation|GetActorLocation (Variables|Default|GetLookAtTarget)) (Math|Vector|MakeVector 0.0 (* (Math|Trig|Cos(Degrees) _returnvalue_3) _distancefromtarget) (* (Math|Trig|Sin(Degrees) _returnvalue_3) _distancefromtarget -1.0))) false false))

(fn ConstructionScript)