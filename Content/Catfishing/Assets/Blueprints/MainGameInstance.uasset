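; Game instance for Catfishing that carries water distortion strength and background music across levels.
; Init caches the Strength parameter of the MPC_WaterDistortion collection, and LevelInit writes it back.
; LevelInit also spawns the music as a 2D sound that persists across level transitions, only when no valid audio component exists.
; MusicVolumeUpdate stores the new volume and applies it to that component.
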(event Custom|LevelInit
  (Rendering|Material|SetScalarParameterValue "/Game/Catfishing/Assets/Materials/MPC_WaterDistortion.MPC_WaterDistortion" "Strength" (Variables|Default|GetWaveDistortionStrength) :!class /Script/Engine.KismetMaterialLibrary)
  (Utilities|IsValid (Variables|Default|GetBgAudioComponent)
    (:Is%20Not%20Valid
      (bind _returnvalue (Audio|SpawnSound2D "/Game/Catfishing/Assets/SoundCues/BackgroundMusic.BackgroundMusic" (Variables|Default|GetMusicVolume) 1.0 0.0 0 true))
      (Variables|Default|SetBgAudioComponent _returnvalue))))

(event Custom|MusicVolumeUpdate
  (params (NewMusicVolume :type Float%20%28double-precision%29))
  (bind _output_get (Variables|Default|SetMusicVolume NewMusicVolume))
  (Audio|Components|Audio|SetVolumeMultiplier (Variables|Default|GetBgAudioComponent) _output_get :!class /Script/Engine.AudioComponent))

(event EventInit
  (bind _returnvalue (Rendering|Material|GetScalarParameterValue "/Game/Catfishing/Assets/Materials/MPC_WaterDistortion.MPC_WaterDistortion" "Strength" :!class /Script/Engine.KismetMaterialLibrary))
  (Variables|Default|SetWaveDistortionStrength _returnvalue))