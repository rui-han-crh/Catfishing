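; Pawn component that gives its owner grid movement and line-of-sight queries on the level's Paper2D tilemap, found at BeginPlay.
; It converts its world location to tile coordinates and treats out-of-bounds or layer-0 "Obstacle" user-data tiles as blocked.
; That check drives single-step move validation, straight row/column sight tests (diagonals always fail), and a first-blocker search that greedily steps along the dominant axis.
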(event EventBeginPlay
  (bind _returnvalue (Actor|GetActorOfClass "/Script/Paper2D.PaperTileMapActor"))
  (Variables|Default|SetTilemap _returnvalue))

(event EventTick
  (params (DeltaSeconds :type Float%20%28single-precision%29)))

(fn WorldtoTilemapPosition
  (bind _returnvalue (Transformation|GetWorldLocation))
  (bind _tilemap (Variables|Default|GetTilemap))
  (bind _tilesize (Variables|Default|GetTileSize))
  (bind _tilesize_2 (Variables|Default|GetTileSize))
  (bind _returnvalue_2 (Math|Conversions|ToFloat(Integer) _tilesize_2))
  (bind _returnvalue_3 (Math|Conversions|ToFloat(Integer) _tilesize_2))
  (bind _returnvalue_4 (Transformation|GetActorLocation _tilemap))
  (bind _returnvalue_5 (* _returnvalue_2 -0.5))
  (bind _returnvalue_6 (* _returnvalue_3 -0.5))
  (bind _returnvalue_7 (Math|Vector|MakeVector _returnvalue_5 _returnvalue_6 0.0))
  (bind _returnvalue_8 (+ _returnvalue_4 _returnvalue_7))
  (bind _returnvalue_9 (- _returnvalue _returnvalue_8))
  (bind (_x _y) (Math|Vector|BreakVector _returnvalue_9))
  (return (Utilities|Struct|MakeIntPoint (Math|Float|Truncate (/ _x _tilesize)) (Math|Float|Truncate (/ _y _tilesize)))))

(fn CheckifValidDirectionfromActor
  (params (Direction :type Vector))
  (bind _tilemapposition (CallFunction|WorldtoTilemapPosition))
  (bind (_isvalidmove _fromposition _toposition) (CallFunction|CheckifValidDirection _tilemapposition Direction))
  (return _isvalidmove _fromposition _toposition))

(fn FindBlockingBetween
  (params (FromPosition :type Int%20Point%20Structure) (ToPosition :type Int%20Point%20Structure))
  (bind _output_get (LocalVariables|SetCurrentPosition FromPosition))
  (while (!= ToPosition (LocalVariables|GetCurrentPosition))
    (if (< (Math|Float|Absolute(Float) (/ (Math|Conversions|ToFloat(Integer) (.y (- ToPosition _output_get))) (Math|Conversions|ToFloat(Integer) (.x (- ToPosition _output_get))))) 1.0)
      (bind (_isvalidmove _fromposition _toposition) (CallFunction|CheckifValidDirection (LocalVariables|GetCurrentPosition) (* (.x (- ToPosition _output_get)) "1.000000,0,0")))
      (if _isvalidmove
        (LocalVariables|SetCurrentPosition _toposition)
        (else
          (return true _toposition)))
      (else
        (bind (_isvalidmove_2 _fromposition_2 _toposition_2) (CallFunction|CheckifValidDirection (LocalVariables|GetCurrentPosition) (* (.y (- ToPosition _output_get)) "0,1.000000,0")))
        (if _isvalidmove_2
          (LocalVariables|SetCurrentPosition _toposition_2)
          (else
            (return true _toposition_2))))))
  (return false ""))

(fn CheckifValidDirection
  (params (TilemapPosition :type Int%20Point%20Structure) (Direction :type Vector))
  (bind _returnvalue (Class|KismetMathLibrary|VectorNormal2D Direction 0.0001))
  (bind _returnvalue_2 (+ (.x TilemapPosition) (.x _returnvalue)))
  (bind _returnvalue_3 (+ (.y TilemapPosition) (.y _returnvalue)))
  (bind _returnvalue_4 (Math|Float|Round _returnvalue_2))
  (bind _returnvalue_5 (Math|Float|Round _returnvalue_3))
  (bind _isblocked (CallFunction|CheckIsBlockedat (Utilities|Struct|MakeIntPoint _returnvalue_4 _returnvalue_5)))
  (return (not _isblocked) TilemapPosition (Utilities|Struct|MakeIntPoint _returnvalue_4 _returnvalue_5)))

(fn CheckifCanSee
  (params (PositionToSee :type Int%20Point%20Structure))
  (bind _tilemapposition (CallFunction|WorldtoTilemapPosition))
  (LocalVariables|SetTilemapPosition _tilemapposition)
  (if (== (.x (- PositionToSee _tilemapposition)) 0)
    (for _index (range (Math|Integer|Min(Integer) (.y (LocalVariables|GetTilemapPosition)) (.y PositionToSee)) (Math|Integer|Max(Integer) (.y (LocalVariables|GetTilemapPosition)) (.y PositionToSee)))
      (bind _isblocked (CallFunction|CheckIsBlockedat (Utilities|Struct|MakeIntPoint (.x (LocalVariables|GetTilemapPosition)) _index)))
      (if _isblocked
        (return false (Math|Vector|MakeVector 0.0 (Math|Conversions|ToFloat(Integer) (- (.y PositionToSee) (.y (LocalVariables|GetTilemapPosition)))) 0.0))))
    (return true (Math|Vector|MakeVector 0.0 (Math|Conversions|ToFloat(Integer) (- (.y PositionToSee) (.y (LocalVariables|GetTilemapPosition)))) 0.0))
    (elif (== (.y (- PositionToSee _tilemapposition)) 0)
      (for _index_2 (range (Math|Integer|Min(Integer) (.x (LocalVariables|GetTilemapPosition)) (.x PositionToSee)) (Math|Integer|Max(Integer) (.x (LocalVariables|GetTilemapPosition)) (.x PositionToSee)))
        (bind _isblocked_2 (CallFunction|CheckIsBlockedat (Utilities|Struct|MakeIntPoint _index_2 (.y (LocalVariables|GetTilemapPosition)))))
        (if _isblocked_2
          (return false (Math|Vector|MakeVector (Math|Conversions|ToFloat(Integer) (- (.x PositionToSee) (.x (LocalVariables|GetTilemapPosition)))) 0.0 0.0))))
      (return true (Math|Vector|MakeVector (Math|Conversions|ToFloat(Integer) (- (.x PositionToSee) (.x (LocalVariables|GetTilemapPosition)))) 0.0 0.0))
      (else
        (return false "0, 0, 0")))))

(fn CheckIsBlockedat
  (params (TilemapPosition :type Int%20Point%20Structure))
  (bind (_mapwidth _mapheight) (Class|PaperTileMapComponent|GetMapSize (Variables|/Script/Paper2D.PaperTileMapActor|GetRenderComponent (Variables|Default|GetTilemap))))
  (return (Math|Boolean|ORBoolean (< (.x TilemapPosition) 0) (>= (.x TilemapPosition) _mapwidth) (< (.y TilemapPosition) 0) (>= (.y TilemapPosition) _mapheight) (== (Class|TileMapBlueprintLibrary|GetTileUserData (Class|PaperTileMapComponent|GetTile (Variables|/Script/Paper2D.PaperTileMapActor|GetRenderComponent (Variables|Default|GetTilemap)) (.x TilemapPosition) (.y TilemapPosition))) "Obstacle"))))