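; Oswald is a player-controlled, grid-based character that moves one tile at a time on a Paper2D tilemap.
; BeginPlay snaps it to its tile center and registers Enhanced Input.
; A stack of held axes lets the most recent press win, and Tick starts the next step once the previous movement stops.
; MoveCharacter validates the direction through TilePawnComponent, announces the move and drives InterpToMovement with relative control points.
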(event Input|EnhancedActionEvents|EnhancedInputActionHorizontal
  (params (ActionValue :type Float%20%28double-precision%29) (ElapsedSeconds :type Float%20%28double-precision%29) (TriggeredSeconds :type Float%20%28double-precision%29) (InputAction :type Input%20Action%20Object%20Reference :default "/Game/Catfishing/Assets/Input/Horizontal.Horizontal"))
  (bind _directionstack (Variables|Default|GetDirectionStack))
  (:Triggered
    (Variables|Default|SetHorizontalActionValue ActionValue))
  (:Started
    (Utilities|Array|Add _directionstack true))
  (:Completed
    (Utilities|Array|RemoveItem _directionstack true)))

(event Input|EnhancedActionEvents|EnhancedInputActionVertical
  (params (ActionValue :type Float%20%28double-precision%29) (ElapsedSeconds :type Float%20%28double-precision%29) (TriggeredSeconds :type Float%20%28double-precision%29) (InputAction :type Input%20Action%20Object%20Reference :default "/Game/Catfishing/Assets/Input/Vertical.Vertical"))
  (bind _directionstack (Variables|Default|GetDirectionStack))
  (:Triggered
    (Variables|Default|SetVerticalActionValue ActionValue))
  (:Started
    (Utilities|Array|Add _directionstack false))
  (:Completed
    (Utilities|Array|RemoveItem _directionstack false)))

(event EventBeginPlay
  (bind _returnvalue (Game|GetPlayerController 0))
  (bind _returnvalue_2 (PlayerController|LocalPlayerSubsystems|GetEnhancedInputLocalPlayerSubsystem _returnvalue))
  (Input|EnableInput (Game|GetPlayerController 0))
  (Actor|GetActorOfClass "/Script/Paper2D.PaperTileMapActor")
  (bind _tilemapposition (Default|WorldtoTilemapPosition (Variables|Default|GetTilePawnComponent)))
  (Transformation|SetActorLocation (Math|Vector|MakeVector (.X (Class|KismetMathLibrary|BreakVector3f (Class|PaperTileMapComponent|GetTileCenterPosition (Variables|/Script/Paper2D.PaperTileMapActor|GetRenderComponent (Variables|/Game/Catfishing/Assets/Blueprints/TilePawnComponent.TilePawnComponent_C|GetTilemap (Variables|Default|GetTilePawnComponent))) (.X (Utilities|Struct|BreakIntPoint _tilemapposition)) (.Y (Utilities|Struct|BreakIntPoint _tilemapposition)) 0 true))) (.Y (Class|KismetMathLibrary|BreakVector3f (Class|PaperTileMapComponent|GetTileCenterPosition (Variables|/Script/Paper2D.PaperTileMapActor|GetRenderComponent (Variables|/Game/Catfishing/Assets/Blueprints/TilePawnComponent.TilePawnComponent_C|GetTilemap (Variables|Default|GetTilePawnComponent))) (.X (Utilities|Struct|BreakIntPoint _tilemapposition)) (.Y (Utilities|Struct|BreakIntPoint _tilemapposition)) 0 true))) (.Z (Class|KismetMathLibrary|BreakVector3f (Transformation|GetActorLocation)))) false false)
  (Utilities|IsValid _returnvalue_2
    (:Is%20Valid
      (Input|AddMappingContext _returnvalue_2 "/Game/Catfishing/Assets/Input/InputMapping.InputMapping" 0 "(bIgnoreAllPressedKeysUntilRelease=True,bForceImmediately=False)"))))

(event EventTick
  (params (DeltaSeconds :type Float%20%28single-precision%29))
  (bind _directionstack (Variables|Default|GetDirectionStack))
  (if (== (Math|Vector|VectorLength (Variables|/Script/Engine.MovementComponent|GetVelocity (Variables|Default|GetInterpToMovement))) 0.0)
    (Variables|Default|SetIsMoving false)
    (if (not (Utilities|Array|IsEmpty _directionstack))
      (if (Utilities|Array|Get(acopy) _directionstack (Utilities|Array|LastIndex _directionstack))
        (CallFunction|MoveCharacter (* (Variables|Default|GetHorizontalActionValue) "1.000000,0,0"))
        (else
          (CallFunction|MoveCharacter (* (Variables|Default|GetVerticalActionValue) "0.000000,-1.000000,0")))))))

(fn ConstructionScript)

(fn MoveCharacter
  (params (Direction :type Vector))
  (bind _interptomovement (Variables|Default|GetInterpToMovement))
  (bind _interptomovement_2 (Variables|Default|GetInterpToMovement))
  (if (not (Variables|Default|GetIsMoving))
    (bind (_isvalidmove _fromposition _toposition) (Default|CheckifValidDirectionfromActor (Variables|Default|GetTilePawnComponent) Direction))
    (if _isvalidmove
      (Variables|Default|SetIsMoving true)
      (Class|InterptoMovementComponent|ResetControlPoints (Variables|Default|GetInterpToMovement))
      (Class|InterptoMovementComponent|AddControlPointPosition _interptomovement "0, 0, 0" true)
      (Class|InterptoMovementComponent|AddControlPointPosition _interptomovement (* Direction (Variables|/Game/Catfishing/Assets/Blueprints/TilePawnComponent.TilePawnComponent_C|GetTileSize (Variables|Default|GetTilePawnComponent))) true)
      (Class|InterptoMovementComponent|FinaliseControlPoints _interptomovement_2)
      (Default|CallOnStartMove _fromposition _toposition)
      (Class|InterptoMovementComponent|RestartMovement _interptomovement_2 1.0))))