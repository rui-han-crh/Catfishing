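; Selector is a level-select tile actor that opens its assigned level when the player, Oswald, lands on it.
; On BeginPlay it makes its mesh visible and binds to Oswald's end-of-move event.
; After each move it compares tile X and Y positions, then opens LevelToPlay on a match.
; Nodes that would hide the mesh and display the level name are disconnected and never run.
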(event Custom|OswaldMoved
  (params (Pawn :type Tilemap%20Pawn%20Object%20Reference) (TilePosition :type Int%20Point%20Structure%20%28by%20ref%29) (Direction :type Vector%20%28by%20ref%29))
  ;[1 1 1] If player is on the selector's tile
  (if (and (== (.x TilePosition) (.x (Variables|Default|GetTilePosition))) (== (.y TilePosition) (.y (Variables|Default|GetTilePosition))))
    ;[1 1 1] Open specific level
    (Game|OpenLevel(byObjectReference) (Variables|Default|GetLevelToPlay))))

(event EventBeginPlay
  (Rendering|SetVisibility (Variables|Default|GetStaticMesh) true false)
  ;[1 1 1] Set player reference
  (bind _returnvalue (Actor|GetActorOfClass "/Game/Catfishing/Assets/Blueprints/Oswald.Oswald_C"))
  ;[1 1 1] Bind player move event
  (EventDispatchers|BindEventtoOnEndMove _returnvalue (delegate Custom|OswaldMoved)))

(fn ConstructionScript)