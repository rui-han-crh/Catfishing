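; A grid-based fish that flees when Oswald ends a move in clear straight-line sight within danger range, exploding if he reaches its tile.
; It glides tile to tile with InterpToMovement, chaining steps until junction, distance or fishnet checks stop it.
; Each step tests forward, left and right, scanning corridors to avoid dead ends and preferring those over fishnets.
; Start, end and action events report its movement.
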(event Custom|BeginMoveSelf
  (params (ImpactResult :type Hit%20Result%20Structure%20%28by%20ref%29) (Time :type Float%20%28single-precision%29))
  (bind _shouldstop (CallFunction|CheckShouldStop (Variables|Default|GetPlayerPosition)))
  (if _shouldstop
    (Default|CallOnEndMove self (Variables|Default|GetTilePosition) (Math|Vector|GetForwardVector (Variables|Default|GetPivot)))
    (Default|CallOnActionFinalize self)
    (elif (Utilities|CheckifMoving)
      (Utilities|FlowControl|DelayUntilNextTick)
      (CallFunction|BeginMoveSelf (Collision|MakeHitResult false false 0.0 0.0 "0, 0, 0" "0, 0, 0" "0,0,1" "0,0,1" 0 0) 0.0)
      (else
        (Default|CallOnActionInitialize self)
        (bind (_initialtileposition _decideddirection) (CallFunction|MoveCharacter (Variables|Default|GetForwardDirection)))
        (Variables|Default|SetForwardDirection _decideddirection)
        (if (Variables|Default|GetJustStartedMoving)
          (Variables|Default|SetJustStartedMoving false)
          (Default|CallOnStartMove self _initialtileposition _decideddirection))))))

(event Custom|PlayerMoved
  (params (Pawn :type Tilemap%20Pawn%20Object%20Reference) (TilePosition :type Int%20Point%20Structure%20%28by%20ref%29) (Direction :type Vector%20%28by%20ref%29))
  (bind _output_get (Variables|Default|SetPlayerPosition TilePosition))
  (Variables|Default|SetForwardDirection (Math|Conversions|ToVector(Vector2D) (Math|Conversions|ToVector2D(IntPoint) (- (Variables|Default|GetTilePosition) TilePosition))))
  (bind (_cansee _direction) (CallFunction|CheckifCanSeePlayer _output_get))
  ;[1 1 1] Can see and within range of player
  (if (and (<= (Math|Vector|VectorLength _direction) (Variables|Default|GetDangerRange)) _cansee)
    ;[1 1 1] Rotate only if not moving
    (if (Utilities|CheckifMoving)
      _
      (else
        (CallFunction|RotateFishtoFaceDirection (* _direction -1.0))))
    (if (Math|Vector|VectorIsZero (* _direction -1.0))
      (Actor|DestroyActor)
      (Effects|SpawnEmitteratLocation "/Game/StarterContent/Particles/P_Explosion.P_Explosion" (Transformation|GetActorLocation))
      (elif (not (Utilities|CheckifMoving))
        (Variables|Default|SetJustStartedMoving true)
        (CallFunction|BeginMoveSelf (Collision|MakeHitResult false false 0.0 0.0 "0, 0, 0" "0, 0, 0" "0,0,1" "0,0,1" 0 0) 0.0)))))

(event EventBeginPlay
  (bind _returnvalue (Actor|GetActorOfClass "/Game/Catfishing/Assets/Blueprints/Oswald.Oswald_C"))
  (EventDispatchers|BindEventtoOnEndMove _returnvalue (delegate Custom|PlayerMoved))
  (EventDispatchers|BindEventtoOnInterptoStop (Variables|Default|GetInterpToMovement) (delegate Custom|BeginMoveSelf))
  (bind _returnvalue_2 (Actor|GetActorOfClass "/Script/Catfishing.CatfishingTilemapActor"))
  (bind _output_get (Variables|Default|SetTilemap _returnvalue_2))
  (bind _tileposition (CallFunction|GetFishTilePosition))
  (bind _output_get_2 (Variables|Default|SetTilePosition _tileposition))
  (Transformation|SetActorLocation (Math|Vector|MakeVector (.x (Class|PaperTileMapComponent|GetTileCenterPosition (Variables|/Script/Paper2D.PaperTileMapActor|GetRenderComponent _output_get) (.x _output_get_2) (.y _output_get_2) 0 true)) (.y (Class|PaperTileMapComponent|GetTileCenterPosition (Variables|/Script/Paper2D.PaperTileMapActor|GetRenderComponent _output_get) (.x _output_get_2) (.y _output_get_2) 0 true)) (.Z (Class|KismetMathLibrary|BreakVector3f (Transformation|GetActorLocation)))) false false))

(fn ConstructionScript)

(fn MoveCharacter
  (params (Direction :type Vector))
  (LocalVariables|Set_InitialTilePosition (Variables|Default|GetTilePosition))
  (LocalVariables|SetNormalizedDirection (Class|KismetMathLibrary|VectorNormal2D Direction 0.0001))
  (Variables|Default|SetNoChoiceDirection "0, 0, 0")
  (bind _array_element (Utilities|Array|ForEachLoopwithBreak (Utilities|Array|MakeArray (LocalVariables|GetNormalizedDirection) (Utilities|RotateLeft (LocalVariables|GetNormalizedDirection)) (Utilities|RotateRight (LocalVariables|GetNormalizedDirection))) :!label _label)
    (:LoopBody
      ;[1 1 1] Is there no wall or dead end in this direction?
      (bind (_canmove _to_position) (CallFunction|TrytoMove _array_element))
      (if _canmove
        ;[1 1 1] Is there a fishnet in this direction?
        (if (Class|CatfishingTilemapActor|HasFishnet (Variables|Default|GetTilemap) (+ (Variables|Default|GetTilePosition) (Utilities|VectortoIntPoint _array_element)))
          ;[1 1 1] Save first feasible but suboptimal direction, only if not set
          (if (Math|Vector|VectorIsZero (LocalVariables|GetSuboptimalDirection))
            (LocalVariables|SetSuboptimalDirection _array_element))
          (else
            (LocalVariables|SetOptimalMove true)
            (goto _label Break)))))
    (:Completed
      (if (LocalVariables|GetOptimalMove)
        (LocalVariables|SetNormalizedDirection _array_element)
        (bind _output_get (Variables|Default|SetTilePosition _to_position))
        (CallFunction|RotateFishtoFaceDirection (LocalVariables|GetNormalizedDirection) :!label _label_2)
        (Class|InterptoMovementComponent|ResetControlPoints (Variables|Default|GetInterpToMovement))
        (Class|InterptoMovementComponent|AddControlPointPosition (Variables|Default|GetInterpToMovement) (Transformation|GetActorLocation) false)
        (Class|InterptoMovementComponent|AddControlPointPosition (Variables|Default|GetInterpToMovement) (Utilities|IntPointtoVectorInheritZ _output_get) false)
        (Class|InterptoMovementComponent|FinaliseControlPoints (Variables|Default|GetInterpToMovement))
        (Class|InterptoMovementComponent|RestartMovement (Variables|Default|GetInterpToMovement) 1.0)
        (return (LocalVariables|Get_InitialTilePosition) (LocalVariables|GetNormalizedDirection))
        (else
          ;[1 1 1] Choose dead end over trap
          (if (not (Math|Vector|VectorIsZero (Variables|Default|GetNoChoiceDirection)))
            (bind _output_get_2 (LocalVariables|SetNormalizedDirection (Variables|Default|GetNoChoiceDirection)))
            (Variables|Default|SetTilePosition (+ (Utilities|VectortoIntPoint _output_get_2) (Variables|Default|GetTilePosition)))
            (goto _label_2)
            (elif (not (Math|Vector|VectorIsZero (LocalVariables|GetSuboptimalDirection)))
              (bind _output_get_3 (LocalVariables|SetNormalizedDirection (LocalVariables|GetSuboptimalDirection)))
              (Variables|Default|SetTilePosition (+ (Utilities|VectortoIntPoint _output_get_3) (Variables|Default|GetTilePosition)))
              (goto _label_2))))))))

(fn TrytoMove
  (params (Forward :type Vector))
  (bind _tileposition (Variables|Default|GetTilePosition))
  (bind _isvaliddirection (CallFunction|CheckifValidDirection _tileposition Forward))
  (if _isvaliddirection
    (bind _iscorridor (CallFunction|CorridorCheck Forward))
    (if _iscorridor
      (if (Math|Vector|VectorIsZero (Variables|Default|GetNoChoiceDirection))
        (Variables|Default|SetNoChoiceDirection Forward))
      (return false "")
      (else
        (return true (+ _tileposition (Utilities|VectortoIntPoint Forward)))))
    (else
      (return false ""))))

(fn CorridorCheck
  (params (Forward :type Vector))
  (LocalVariables|SetDistanceSoFar 1)
  (while (not (LocalVariables|GetIsAtEnd))
    ;[1 1 1] Left Check (Is there a blocking object on the left side?)
    (bind _isvaliddirection (CallFunction|CheckifValidDirection (+ (Utilities|VectortoIntPoint (* Forward (LocalVariables|GetDistanceSoFar))) (Variables|Default|GetTilePosition)) (Utilities|RotateLeft (Class|KismetMathLibrary|VectorNormal2D (* Forward (LocalVariables|GetDistanceSoFar)) 0.0001))))
    ;;[1 1 1] Is there a fishnet diagonally left?
    (if (== (LocalVariables|GetDistanceSoFar) 1)
      (if (and (not (Class|CatfishingTilemapActor|HasFishnet (Variables|Default|GetTilemap) (+ (+ (Utilities|VectortoIntPoint (* Forward (LocalVariables|GetDistanceSoFar))) (Variables|Default|GetTilePosition)) (Utilities|VectortoIntPoint (Utilities|RotateLeft (Class|KismetMathLibrary|VectorNormal2D (* Forward (LocalVariables|GetDistanceSoFar)) 0.0001)))))) _isvaliddirection)
        (return false)
        (else
          _))
      (elif _isvaliddirection
        (return false)
        (else
          _)))
    ;[1 1 1] Right Check (Is there a blocking tile on the right side?)
    (bind _isvaliddirection_2 (CallFunction|CheckifValidDirection (+ (Utilities|VectortoIntPoint (* Forward (LocalVariables|GetDistanceSoFar))) (Variables|Default|GetTilePosition)) (Utilities|RotateRight (Class|KismetMathLibrary|VectorNormal2D (* Forward (LocalVariables|GetDistanceSoFar)) 0.0001))))
    ;;[1 1 1] Is there a fishnet diagonally right?
    (if (== (LocalVariables|GetDistanceSoFar) 1)
      (if (and (not (Class|CatfishingTilemapActor|HasFishnet (Variables|Default|GetTilemap) (+ (+ (Utilities|VectortoIntPoint (* Forward (LocalVariables|GetDistanceSoFar))) (Variables|Default|GetTilePosition)) (Utilities|VectortoIntPoint (Utilities|RotateRight (Class|KismetMathLibrary|VectorNormal2D (* Forward (LocalVariables|GetDistanceSoFar)) 0.0001)))))) _isvaliddirection_2)
        (return false)
        (else
          _))
      (elif _isvaliddirection_2
        (return false)
        (else
          _)))
    ;[1 1 1] Forward Check (Is there a blocking tile or a fishnet ahead?)
    (bind _isvaliddirection_3 (CallFunction|CheckifValidDirection (+ (Utilities|VectortoIntPoint (* Forward (LocalVariables|GetDistanceSoFar))) (Variables|Default|GetTilePosition)) (Class|KismetMathLibrary|VectorNormal2D (* Forward (LocalVariables|GetDistanceSoFar)) 0.0001)))
    (if (and _isvaliddirection_3 (not (Class|CatfishingTilemapActor|HasFishnet (Variables|Default|GetTilemap) (+ (Utilities|VectortoIntPoint (* Forward (LocalVariables|GetDistanceSoFar))) (Variables|Default|GetTilePosition)))))
      (Math|Integer|IncrementInt (LocalVariables|GetDistanceSoFar)) ; Increase straight line distance
      (else
        (LocalVariables|SetIsAtEnd true) ; We are at the end of the corridor
      )))
  (return true))

(fn CheckShouldStop
  (params (PlayerPosition :type Int%20Point%20Structure))
  (bind _pivot (Variables|Default|GetPivot))
  (bind _returnvalue (Math|Vector|GetForwardVector _pivot))
  (if (Class|CatfishingTilemapActor|HasFishnet (Variables|Default|GetTilemap) (Variables|Default|GetTilePosition))
    (Development|PrintString "Trapped")
    ;[1 1 1] Trapped in Fishnet
    (return true)
    (else
      (bind _output_get (LocalVariables|SetDistanceFromPlayer (Math|Vector|Distance2D(Vector) (Math|Conversions|ToVector2D(IntPoint) (Variables|Default|GetTilePosition)) (Math|Conversions|ToVector2D(IntPoint) PlayerPosition))))
      (bind _output_get_2 (LocalVariables|SetInSight (Class|CatfishingTilemapActor|IsStraightLine (Variables|Default|GetTilemap) (Variables|Default|GetTilePosition) PlayerPosition)))
      ;[1 1 1] At least 2 directions are valid to move
      (bind _isvaliddirection (CallFunction|CheckifValidDirection (Variables|Default|GetTilePosition) (Utilities|RotateRight _returnvalue)))
      (bind _isvaliddirection_2 (CallFunction|CheckifValidDirection (Variables|Default|GetTilePosition) (Utilities|RotateLeft _returnvalue)))
      (bind _isvaliddirection_3 (CallFunction|CheckifValidDirection (Variables|Default|GetTilePosition) _returnvalue))
      (return (or (and (or (>= (+ (Math|Conversions|ToInteger(Boolean) _isvaliddirection) (Math|Conversions|ToInteger(Boolean) _isvaliddirection_2) (Math|Conversions|ToInteger(Boolean) _isvaliddirection_3)) 2) (not _isvaliddirection_3)) (or (not _output_get_2) (> _output_get 2.0))) (and (LocalVariables|GetInSight) (>= (LocalVariables|GetDistanceFromPlayer) 6.0)))))))

(fn RotateFishtoFaceDirection
  (params (Direction :type Vector))
  (Transformation|SetWorldRotation (Variables|Default|GetPivot) (Math|Rotator|FindLookatRotation (Transformation|GetWorldLocation (Variables|Default|GetPivot)) (+ (Transformation|GetWorldLocation (Variables|Default|GetPivot)) Direction)) false false))

(fn FindFirstValidDirection
  (params (Direction :type Vector))
  (bind _rotated_vector (Utilities|RotateLeft Direction))
  (bind _rotated_vector_2 (Utilities|RotateRight Direction))
  (bind _isvaliddirection (CallFunction|CheckifValidDirection (Variables|Default|GetTilePosition) Direction))
  (if _isvaliddirection
    (return (+ (Variables|Default|GetTilePosition) (Utilities|VectortoIntPoint Direction)) Direction)
    (else
      (bind _isvaliddirection_2 (CallFunction|CheckifValidDirection (Variables|Default|GetTilePosition) _rotated_vector))
      (if _isvaliddirection_2
        (return (+ (Variables|Default|GetTilePosition) (Utilities|VectortoIntPoint _rotated_vector)) _rotated_vector)
        (else
          (bind _isvaliddirection_3 (CallFunction|CheckifValidDirection (Variables|Default|GetTilePosition) _rotated_vector_2))
          (if _isvaliddirection_3
            (return (+ (Variables|Default|GetTilePosition) (Utilities|VectortoIntPoint _rotated_vector_2)) _rotated_vector_2)
            (else
              (return "" "0, 0, 0"))))))))

(fn FindFirstValidDirectionfromForward
  (bind (_toposition _validdirection) (CallFunction|FindFirstValidDirection (Math|Vector|GetForwardVector (Variables|Default|GetPivot))))
  (return _toposition _validdirection))

(fn GetFishTilePosition
  (bind _returnvalue (Class|CatfishingTilemapActor|WorldtoTilePosition (Variables|Default|GetTilemap) (Transformation|GetActorLocation)))
  (return _returnvalue))

(fn CheckifCanSeePlayer
  (params (ToSeePosition :type Int%20Point%20Structure))
  (bind _tileposition (CallFunction|GetFishTilePosition))
  (bind _returnvalue (Class|CatfishingTilemapActor|CheckifAnyBlockedTiles (Variables|Default|GetTilemap) _tileposition ToSeePosition))
  (return (and (not _returnvalue) (Class|CatfishingTilemapActor|IsStraightLine (Variables|Default|GetTilemap) _tileposition ToSeePosition)) (Math|Conversions|ToVector(Vector2D) (- ToSeePosition _tileposition))))

(fn CheckifValidDirection
  (params (StartTile :type Int%20Point%20Structure) (Direction :type Vector))
  (bind _returnvalue (Class|CatfishingTilemapActor|CheckifValidDirection (Variables|Default|GetTilemap) StartTile Direction))
  (return _returnvalue))