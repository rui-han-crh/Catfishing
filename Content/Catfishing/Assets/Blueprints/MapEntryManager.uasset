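; Level manager that runs Oswald's entry and exit cutscenes and gates the exit Selector on clearing all Fish.
; BeginPlay disables the Selector, lowers Oswald into place and spawns a hidden anchor rope above the exit.
; UpdateState drops the anchor when no Fish remain, and the anchor stopping activates the Selector.
; Entering it hoists Oswald on the cable before opening the next level; both cutscenes animate through self-calling next-tick loops.
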(event Custom|UpdateState
  (bind _outactors (Actor|GetAllActorsOfClass "/Game/Catfishing/Assets/Blueprints/Fish.Fish_C"))
  (if (== (Utilities|Array|Length _outactors) 0)
    (CallFunction|DropAnchoratExit)
    (EventDispatchers|BindEventtoOnAnchorStop (Variables|Default|GetAnchorRopeActor) (delegate Custom|EnableSelector))))

(event Custom|PlayEndingCutscene
  (params (Pawn :type Tilemap%20Pawn%20Object%20Reference))
  (bind _anchorropeactor (Variables|Default|GetAnchorRopeActor))
  (bind _cable (Variables|/Game/Catfishing/Assets/Blueprints/AnchorRope.AnchorRope_C|GetCable _anchorropeactor))
  (bind _asoswald (Utilities|Casting|CastToOswald Pawn))
  (Default|DisableInputControl _asoswald)
  (Class|CableComponent|SetAttachEndto _cable _asoswald "Pivot" "None")
  (Variables|/Script/CableComponent.CableComponent|SetEndLocation _cable "0, 0, 0")
  (Components|Activation|Activate (Variables|/Game/Catfishing/Assets/Blueprints/Oswald.Oswald_C|GetNS_Bubbles _asoswald) false)
  (CallFunction|EndingCutsceneUpdate)
  (Utilities|FlowControl|Delay 3.0)
  (Variables|Default|SetHasEnded true)
  (Default|OpenLevel (Variables|Default|GetExitPawn)))

(event Custom|EndingCutsceneUpdate
  (bind _returnvalue (Utilities|Time|GetWorldDeltaSeconds))
  (bind _anchorropeactor (Variables|Default|GetAnchorRopeActor))
  (bind _returnvalue_2 (* _returnvalue 8e+01))
  (bind _cable (Variables|/Game/Catfishing/Assets/Blueprints/AnchorRope.AnchorRope_C|GetCable _anchorropeactor))
  (Transformation|SetWorldLocation (Variables|/Script/Catfishing.TilemapPawn|GetPivot (stale Custom|PlayEndingCutscene Pawn)) (Math|Vector|MakeVector (.x (Transformation|GetWorldLocation (Variables|/Script/Catfishing.TilemapPawn|GetPivot (stale Custom|PlayEndingCutscene Pawn)))) (.y (Transformation|GetWorldLocation (Variables|/Script/Catfishing.TilemapPawn|GetPivot (stale Custom|PlayEndingCutscene Pawn)))) (+ (.z (Transformation|GetWorldLocation (Variables|/Script/Catfishing.TilemapPawn|GetPivot (stale Custom|PlayEndingCutscene Pawn)))) _returnvalue_2)) false false)
  (Variables|/Script/CableComponent.CableComponent|SetCableLength _cable (- (Variables|/Script/CableComponent.CableComponent|GetCableLength _cable) _returnvalue_2))
  (if (not (Variables|Default|GetHasEnded))
    (Utilities|FlowControl|DelayUntilNextTick)
    (CallFunction|EndingCutsceneUpdate)))

(event Custom|PlayOpeningCutscene
  (bind _returnvalue (Actor|GetActorOfClass "/Game/Catfishing/Assets/Blueprints/Oswald.Oswald_C"))
  (Components|Activation|Activate (Variables|/Game/Catfishing/Assets/Blueprints/Oswald.Oswald_C|GetNS_Bubbles _returnvalue) false)
  (Default|DisableInputControl _returnvalue)
  (Transformation|SetWorldLocation (Variables|/Script/Catfishing.TilemapPawn|GetPivot _returnvalue) (Math|Vector|MakeVector (.x (Transformation|GetWorldLocation (Variables|/Script/Catfishing.TilemapPawn|GetPivot _returnvalue))) (.y (Transformation|GetWorldLocation (Variables|/Script/Catfishing.TilemapPawn|GetPivot _returnvalue))) (+ (.z (Transformation|GetWorldLocation (Variables|/Script/Catfishing.TilemapPawn|GetPivot _returnvalue))) 3e+02)) false false)
  (CallFunction|OpeningCutsceneUpdate))

(event Custom|OpeningCutsceneUpdate
  (Transformation|SetWorldLocation (Variables|/Script/Catfishing.TilemapPawn|GetPivot (stale Custom|PlayOpeningCutscene _returnvalue)) (Math|Vector|MakeVector (.x (Transformation|GetWorldLocation (Variables|/Script/Catfishing.TilemapPawn|GetPivot (stale Custom|PlayOpeningCutscene _returnvalue)))) (.y (Transformation|GetWorldLocation (Variables|/Script/Catfishing.TilemapPawn|GetPivot (stale Custom|PlayOpeningCutscene _returnvalue)))) (+ (.z (Transformation|GetWorldLocation (Variables|/Script/Catfishing.TilemapPawn|GetPivot (stale Custom|PlayOpeningCutscene _returnvalue)))) (* (Utilities|Time|GetWorldDeltaSeconds) -8e+01))) false false)
  (if (<= (.z (Variables|/Script/Engine.SceneComponent|GetRelativeLocation (Variables|/Script/Catfishing.TilemapPawn|GetPivot (stale Custom|PlayOpeningCutscene _returnvalue)))) 1.0)
    (Transformation|SetRelativeLocation (Variables|/Script/Catfishing.TilemapPawn|GetPivot (stale Custom|PlayOpeningCutscene _returnvalue)) "0, 0, 0" false false)
    (Components|Activation|Deactivate (Variables|/Game/Catfishing/Assets/Blueprints/Oswald.Oswald_C|GetNS_Bubbles (stale Custom|PlayOpeningCutscene _returnvalue)))
    (Default|EnableInputControl (stale Custom|PlayOpeningCutscene _returnvalue))
    (else
      (Utilities|FlowControl|DelayUntilNextTick)
      (CallFunction|OpeningCutsceneUpdate))))

(event Custom|EnableSelector
  (Variables|/Game/Catfishing/Assets/Blueprints/Selector.Selector_C|SetIsActive (Variables|Default|GetExitPawn) true))

(event EventBeginPlay
  (bind _returnvalue (Actor|GetActorOfClass "/Game/Catfishing/Assets/Blueprints/Selector.Selector_C"))
  (bind _output_get (Variables|Default|SetExitPawn _returnvalue))
  (Variables|/Game/Catfishing/Assets/Blueprints/Selector.Selector_C|SetIsActive _output_get false)
  (EventDispatchers|BindEventtoOnEnterSelectorTile _output_get (delegate Custom|PlayEndingCutscene))
  (CallFunction|UpdateState)
  (CallFunction|PlayOpeningCutscene)
  (bind _returnvalue_2 (Game|SpawnActorfromClass "/Game/Catfishing/Assets/Blueprints/AnchorRope.AnchorRope_C" (Math|Transform|MakeTransform (Math|Vector|MakeVector (.x (Transformation|GetActorLocation (Variables|Default|GetExitPawn))) (.y (Transformation|GetActorLocation (Variables|Default|GetExitPawn))) (+ (.z (Transformation|GetActorLocation (Variables|Default|GetExitPawn))) 3e+02)) "0, 0, 0" "1.000000,1.000000,1.000000") "Undefined" 0 0))
  (bind _output_get_2 (Variables|Default|SetAnchorRopeActor _returnvalue_2))
  (Rendering|SetActorHiddenInGame _output_get_2 true)
  (Physics|SetSimulatePhysics (Variables|/Game/Catfishing/Assets/Blueprints/AnchorRope.AnchorRope_C|GetAnchor _output_get_2) false))

(fn ConstructionScript)

(fn DropAnchoratExit
  (Rendering|SetActorHiddenInGame (Variables|Default|GetAnchorRopeActor) false)
  (Physics|SetSimulatePhysics (Variables|/Game/Catfishing/Assets/Blueprints/AnchorRope.AnchorRope_C|GetAnchor (Variables|Default|GetAnchorRopeActor)) true))