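; DialogueActor is an actor that plays a sequence of dialogue in a UW_Dialogue widget, optionally showing it at BeginPlay.
; It holds an array of containers, each with a speaker name, avatar and list of lines, tracked by two indices.
; While the widget is shown, any key press advances to the next line or container, updating the widget directly, and hides it after the last one.
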(event EventBeginPlay
  (bind _returnvalue (UserInterface|CreateWidget "/Game/Catfishing/Assets/Blueprints/UW_Dialogue.UW_Dialogue_C" (Game|GetPlayerController 0)))
  (Variables|Default|SetDialogueUI _returnvalue)
  (Input|EnableInput (Game|GetPlayerController 0))
  (if (Variables|Default|GetShowOnBegin)
    (CallFunction|ShowDialogue)))

(event Input|KeyboardEvents|AnyKey
  (params (Key :type Key%20Structure :default "None"))
  (:Pressed
    (if (Variables|Default|GetIsDialogueUIShown)
      (bind _hasended (CallFunction|NextDialogue))
      (if _hasended
        (CallFunction|HideDialogue)))))

(fn ConstructionScript)

(fn ShowDialogue
  (bind _currentdialoguecontainerindex (Variables|Default|GetCurrentDialogueContainerIndex))
  (bind _dialogue (Variables|Default|GetDialogue))
  (bind _output (Utilities|Array|Get(acopy) _dialogue _currentdialoguecontainerindex))
  (bind (_name _avatar _content) (Utilities|Struct|BreakDialogueContainer _output))
  (if (not (Variables|Default|GetIsDialogueUIShown))
    (UserInterface|Viewport|AddtoViewport (Variables|Default|GetDialogueUI) 0)
    (Variables|Default|SetIsDialogueUIShown true)
    (Rendering|Components|TextRender|SetText (Variables|/Game/Catfishing/Assets/Blueprints/UW_Dialogue.UW_Dialogue_C|GetName (Variables|Default|GetDialogueUI)) (Utilities|Text|ToText(String) _name))
    (Variables|/Game/Catfishing/Assets/Blueprints/UW_Dialogue.UW_Dialogue_C|SetAvatar (Variables|Default|GetDialogueUI) _avatar)
    (Rendering|Components|TextRender|SetText (Variables|/Game/Catfishing/Assets/Blueprints/UW_Dialogue.UW_Dialogue_C|GetSpeechText (Variables|Default|GetDialogueUI)) (Utilities|Text|ToText(String) (Utilities|Array|Get(acopy) _content (Variables|Default|GetCurrentDialogueContentIndex))))))

(fn HideDialogue
  (if (Variables|Default|GetIsDialogueUIShown)
    (Variables|Default|SetIsDialogueUIShown false)
    (Widget|RemovefromParent (Variables|Default|GetDialogueUI))))

(fn NextDialogue
  (bind _dialogue (Variables|Default|GetDialogue))
  (bind _currentdialoguecontainerindex (Variables|Default|GetCurrentDialogueContainerIndex))
  (bind _dialogue_2 (Variables|Default|GetDialogue))
  (bind _dialogueui (Variables|Default|GetDialogueUI))
  (bind _currentdialoguecontainerindex_2 (Variables|Default|GetCurrentDialogueContainerIndex))
  (bind _output (Utilities|Array|Get(acopy) _dialogue_2 _currentdialoguecontainerindex_2))
  (bind _output_2 (Utilities|Array|Get(acopy) _dialogue _currentdialoguecontainerindex))
  (bind _result (Math|Integer|IncrementInt (Variables|Default|GetCurrentDialogueContentIndex))
    (:%20%20
      ;[1 1 1] Is it the end of the content in the container?
      (if (>= _result (Utilities|Array|Length (.content _output_2)))
        ;[1 1 1] Go to next container
        (bind _result_2 (Math|Integer|IncrementInt (Variables|Default|GetCurrentDialogueContainerIndex))
          (:%20%20
            ;[1 1 1] Is it also the end of all the containers?
            (if (>= _result_2 (Utilities|Array|Length (Variables|Default|GetDialogue)))
              (return true)
              (else
                (bind _output_get (Variables|Default|SetCurrentDialogueContentIndex 0))
                (Rendering|Components|TextRender|SetText (Variables|/Game/Catfishing/Assets/Blueprints/UW_Dialogue.UW_Dialogue_C|GetName _dialogueui) (Utilities|Text|ToText(String) (.name _output)))
                (Variables|/Game/Catfishing/Assets/Blueprints/UW_Dialogue.UW_Dialogue_C|SetAvatar _dialogueui (.avatar _output))
                (Rendering|Components|TextRender|SetText (Variables|/Game/Catfishing/Assets/Blueprints/UW_Dialogue.UW_Dialogue_C|GetSpeechText _dialogueui) (Utilities|Text|ToText(String) (Utilities|Array|Get(acopy) (.content _output) _output_get)))
                (return false)))))
        (else
          (Rendering|Components|TextRender|SetText (Variables|/Game/Catfishing/Assets/Blueprints/UW_Dialogue.UW_Dialogue_C|GetSpeechText (Variables|Default|GetDialogueUI)) (Utilities|Text|ToText(String) (Utilities|Array|Get(acopy) (.content _output_2) (Variables|Default|GetCurrentDialogueContentIndex)))))))))