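; Camera actor that orbits vertically around a pivot on the Catfishing tilemap, with scroll input setting its tilt.
; BeginPlay computes the pivot from the map's corner and size, stores its distance to it, faces it, and adds the HUD widget.
; Scroll input adjusts a clamped target pitch.
; Tick eases pitch toward that target and uses sine and cosine to reposition the camera on a fixed-radius arc in the Y-Z plane.
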(event Input|EnhancedActionEvents|EnhancedInputActionScroll
  (params (ActionValue :type Float%20%28double-precision%29) (ElapsedSeconds :type Float%20%28double-precision%29) (TriggeredSeconds :type Float%20%28double-precision%29) (InputAction :type Input%20Action%20Object%20Reference :default "/Game/Catfishing/Assets/Input/Scroll.Scroll"))
  (:Triggered
    (Variables|Default|SetDestinationPitchAngle (Math|Float|ClampAngle (- (Variables|Default|GetDestinationPitchAngle) (* ActionValue (Variables|Default|GetScrollSensitivity) -1.0)) (Variables|Default|GetMinAngle) (Variables|Default|GetMaxAngle)))))

(event EventBeginPlay
  (bind _returnvalue (Transformation|GetActorLocation))
  (bind _returnvalue_2 (Transformation|GetActorRotation))
  (bind (_roll _pitch _yaw) (Math|Rotator|BreakRotator _returnvalue_2))
  (bind _returnvalue_3 (Actor|GetActorOfClass "/Script/Catfishing.CatfishingTilemapActor"))
  (bind (_mapwidth _mapheight) (Class|PaperTileMapComponent|GetMapSize (Variables|/Script/Paper2D.PaperTileMapActor|GetRenderComponent _returnvalue_3)))
  (bind _output_get (Variables|Default|SetPivot (+ (Class|PaperTileMapComponent|GetTileCornerPosition (Variables|/Script/Paper2D.PaperTileMapActor|GetRenderComponent _returnvalue_3) 0 0 0 true) (Math|Vector|MakeVector (* _mapwidth 16) (* _mapheight 16) 0.0))))
  (Variables|Default|SetDistanceFromTarget (Math|Vector|Distance(Vector) _returnvalue _output_get))
  (Variables|Default|SetDestinationPitchAngle (* (.Pitch (Math|Rotator|BreakRotator (Math|Rotator|FindLookatRotation _returnvalue _output_get))) -1.0))
  (Transformation|SetActorRotation (Math|Rotator|MakeRotator _roll (.Pitch (Math|Rotator|BreakRotator (Math|Rotator|FindLookatRotation _returnvalue _output_get))) _yaw))
  (bind _returnvalue_4 (UserInterface|CreateWidget "/Game/Catfishing/Assets/Blueprints/UW_Hud.UW_Hud_C" (Game|GetPlayerController 0)))
  (UserInterface|Viewport|AddtoViewport _returnvalue_4 0))

(event EventTick
  (params (DeltaSeconds :type Float%20%28single-precision%29))
  (bind _returnvalue (Transformation|GetActorRotation))
  (bind _destinationpitchangle (Variables|Default|GetDestinationPitchAngle))
  (bind _cameraspeed (Variables|Default|GetCameraSpeed))
  (bind _distancefromtarget (Variables|Default|GetDistanceFromTarget))
  (bind (_roll _pitch _yaw) (Math|Rotator|BreakRotator _returnvalue))
  (bind _returnvalue_2 (* _destinationpitchangle -1.0))
  (bind _returnvalue_3 (Math|Interpolation|FInterpTo _pitch _returnvalue_2 DeltaSeconds _cameraspeed))
  (Transformation|SetActorRotation (Math|Rotator|MakeRotator _roll _returnvalue_3 _yaw))
  (Transformation|SetActorLocation (+ (Variables|Default|GetPivot) (Math|Vector|MakeVector 0.0 (* (Math|Trig|Cos(Degrees) _returnvalue_3) _distancefromtarget) (* (Math|Trig|Sin(Degrees) _returnvalue_3) _distancefromtarget -1.0))) false false))

(fn ConstructionScript)