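; StateManager provides undo and restart for the tilemap game by snapshotting tile data and pawn positions and rotations.
; Pawn action events record each mover's starting state, pushing the snapshot onto a stack once all finish.
; Undo pops that stack and Restart reapplies the initial state, both only while pawns are idle.
; Restoring rebuilds Oswald's fishnet actors from tile flags and repositions saved pawns.
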(event Custom|PawnActionInitialized
  (params (Pawn :type Tilemap%20Pawn%20Object%20Reference))
  (Utilities|Set|Add (Variables|Default|GetAwaitingStopRegistry) Pawn)
  (CallFunction|AddPawnStatetoCurrentState Pawn))

(event Custom|PawnActionFinalized
  (params (Pawn :type Tilemap%20Pawn%20Object%20Reference))
  (Utilities|Set|Remove (Variables|Default|GetAwaitingStopRegistry) Pawn)
  (if (== (Utilities|Set|Length (Variables|Default|GetAwaitingStopRegistry)) 0)
    (CallFunction|SaveCurrentStateIntoStack)
    (CallFunction|CreateNewMapState)))

(event Input|EnhancedActionEvents|EnhancedInputActionUndo
  (params (ActionValue :type Boolean) (ElapsedSeconds :type Float%20%28double-precision%29) (TriggeredSeconds :type Float%20%28double-precision%29) (InputAction :type Input%20Action%20Object%20Reference :default "/Game/Catfishing/Assets/Input/Undo.Undo"))
  (bind _mapstatestack (Variables|Default|GetMapStateStack))
  (bind _mapstatestack_2 (Variables|Default|GetMapStateStack))
  (bind _returnvalue (Utilities|Array|LastIndex _mapstatestack))
  (bind _output (Utilities|Array|Get(acopy) _mapstatestack _returnvalue))
  (:Triggered
    ;[1 1 1] Ignore command if nothing in stack
    (if (not (Utilities|Array|IsEmpty (Variables|Default|GetMapStateStack)))
      ;[1 1 1] Ignore command if characters are still moving
      (if (Utilities|Set|IsEmpty (Variables|Default|GetAwaitingStopRegistry))
        (CallFunction|RestoreStatefromStack (.maptiledata _output) (.tilepawndata _output))
        ;[1 1 1] Pop out the last saved state
        (Utilities|Array|RemoveIndex _mapstatestack_2 (Utilities|Array|LastIndex _mapstatestack_2))
        (CallFunction|CreateNewMapState)))))

(event Input|EnhancedActionEvents|EnhancedInputActionRestart
  (params (ActionValue :type Boolean) (ElapsedSeconds :type Float%20%28double-precision%29) (TriggeredSeconds :type Float%20%28double-precision%29) (InputAction :type Input%20Action%20Object%20Reference :default "/Game/Catfishing/Assets/Input/Restart.Restart"))
  (bind _initialfullmapstate (Variables|Default|GetInitialFullMapState))
  (:Triggered
    ;[1 1 1] Ignore command if characters are still moving
    (if (Utilities|Set|IsEmpty (Variables|Default|GetAwaitingStopRegistry))
      (CallFunction|RestoreStatefromStack (.maptiledata _initialfullmapstate) (.tilepawndata _initialfullmapstate))
      ;[1 1 1] Clear the stack to simulate restart
      (Utilities|Array|Clear (Variables|Default|GetMapStateStack))
      (CallFunction|CreateNewMapState))))

(event EventBeginPlay
  (Utilities|FlowControl|Delay 1.0)
  (bind _returnvalue (Actor|GetActorOfClass "/Script/Catfishing.CatfishingTilemapActor"))
  (Variables|Default|SetTilemap _returnvalue)
  (Input|EnableInput (Game|GetPlayerController 0))
  (CallFunction|CreateNewMapState)
  ;[1 1 1] Oswald keeps the nets
  (bind _returnvalue_2 (Actor|GetActorOfClass "/Game/Catfishing/Assets/Blueprints/Oswald.Oswald_C"))
  (Variables|Default|SetOswald _returnvalue_2)
  (bind _outactors (Actor|GetAllActorsOfClass "/Script/Catfishing.TilemapPawn"))
  (for _array_element _outactors
    (EventDispatchers|BindEventtoOnActionInitialize _array_element (delegate Custom|PawnActionInitialized))
    (EventDispatchers|BindEventtoOnActionFinalize _array_element (delegate Custom|PawnActionFinalized)))
  (Utilities|FlowControl|DelayUntilNextTick) ; Avoids some strange race condition
  (bind _outactors_2 (Actor|GetAllActorsOfClass "/Script/Catfishing.TilemapPawn"))
  (for _array_element_2 _outactors_2
    (CallFunction|AddPawnStatetoCurrentState _array_element_2))
  (Variables|Default|SetInitialFullMapState (Variables|Default|GetCurrentMapState))
  (CallFunction|CreateNewMapState))

(fn ConstructionScript)

(fn DeleteAllFishnets
  (bind _values (Utilities|Map|Values (Variables|/Game/Catfishing/Assets/Blueprints/Oswald.Oswald_C|GetFishnets (Variables|Default|GetOswald))))
  (for _array_element _values
    (Actor|DestroyActor _array_element))
  (Variables|/Game/Catfishing/Assets/Blueprints/Oswald.Oswald_C|SetFishnets (Variables|Default|GetOswald) (Utilities|Map|MakeMap)))

(fn ReconstructFishnetsfromState
  (params (MapTileData :type Array%20of%20Tile%20Data%20Structures))
  (for (_array_element _array_index) MapTileData
    (if (Utilities|Struct|BreakTileData _array_element)
      (bind _mapwidth (Class|PaperTileMapComponent|GetMapSize (Variables|/Script/Paper2D.PaperTileMapActor|GetRenderComponent (Variables|Default|GetTilemap))))
      (bind _returnvalue (Game|SpawnActorfromClass "/Game/Catfishing/Assets/Blueprints/Fishnet.Fishnet_C" (Math|Conversions|ToTransform(Vector) (Class|PaperTileMapComponent|GetTileCenterPosition (Variables|/Script/Paper2D.PaperTileMapActor|GetRenderComponent (Variables|Default|GetTilemap)) (Math|Integer|%(Integer) _array_index _mapwidth) (/ _array_index _mapwidth) 0 true)) "Undefined" 0 0))
      (Utilities|Map|Add (Variables|/Game/Catfishing/Assets/Blueprints/Oswald.Oswald_C|GetFishnets (Variables|Default|GetOswald)) _array_index _returnvalue))))

(fn SaveCurrentStateIntoStack
  ;[1 1 1] Save the map state into the stack
  (Utilities|Array|Add (Variables|Default|GetMapStateStack) (Variables|Default|GetCurrentMapState)))

(fn CreateNewMapState
  (bind (_mapwidth _mapheight) (Class|PaperTileMapComponent|GetMapSize (Variables|/Script/Paper2D.PaperTileMapActor|GetRenderComponent (Variables|Default|GetTilemap))))
  ;[1 1 1] Create a new map state for the current progress
  (Utilities|Array|Resize (Class|CatfishingTilemapActor|GetMapTileData (Variables|Default|GetTilemap)) (* _mapwidth _mapheight))
  (Utilities|Struct|SetmembersinMapState (Variables|Default|GetCurrentMapState) (Class|CatfishingTilemapActor|GetMapTileData (Variables|Default|GetTilemap)) (Utilities|Map|MakeMap)))

(fn RestoreStatefromStack
  (params (MapTileData :type Array%20of%20Tile%20Data%20Structures) (TilemapPawnKeys :type Map%20of%20Tilemap%20Pawn%20Object%20References%20to%20Structs))
  (bind _keys (Utilities|Map|Keys TilemapPawnKeys))
  (CallFunction|DeleteAllFishnets)
  (Class|CatfishingTilemapActor|SetMapTileData (Variables|Default|GetTilemap) MapTileData)
  (CallFunction|ReconstructFishnetsfromState MapTileData)
  (for _array_element _keys
    (Utilities|IsValid _array_element
      (:Is%20Valid
        (Variables|/Script/Catfishing.TilemapPawn|SetTilePosition _array_element (.tileposition (.Value (Utilities|Map|Find TilemapPawnKeys _array_element))))
        (Transformation|SetActorLocation _array_element (.location (.transform (.Value (Utilities|Map|Find TilemapPawnKeys _array_element)))) false false)
        (Transformation|SetWorldRotation (Variables|/Script/Catfishing.TilemapPawn|GetPivot _array_element) (.rotation (.transform (.Value (Utilities|Map|Find TilemapPawnKeys _array_element)))) false false)))))

(fn AddPawnStatetoCurrentState
  (params (Pawn :type Tilemap%20Pawn%20Object%20Reference))
  (bind _currentmapstate (Variables|Default|GetCurrentMapState))
  (bind _tilepawndata (Utilities|Struct|BreakMapState _currentmapstate))
  (if (not (.ReturnValue (Utilities|Map|Find _tilepawndata Pawn)))
    (Utilities|Map|Add _tilepawndata Pawn (Utilities|Struct|MakeTilePositionAndTransform (Variables|/Script/Catfishing.TilemapPawn|GetTilePosition Pawn) (Math|Transform|MakeTransform (Transformation|GetActorLocation Pawn) (Transformation|GetWorldRotation (Variables|/Script/Catfishing.TilemapPawn|GetPivot Pawn)) "1.000000,1.000000,1.000000")))))